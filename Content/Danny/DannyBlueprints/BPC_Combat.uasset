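; Player combat component for BP_ThirdPersonCharacter, covering sword combos, target lock-on and stamina drain.
; Attack presses during the montage queue combos, which montage notifies continue or cut short.
; Lock-on toggles via a camera-forward sphere trace, attaches a marker actor and steers control rotation toward the target on Tick.
; A looping-timer sphere trace along the blade applies throttled damage, while separate stamina events drain a clamped value and flag exhaustion at zero.
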(event Custom|ConsumeStaminaAction
  ;[0.15 0.15 0.15] Stamina
  (if (not (Variables|Default|GetIsExhausted))
    (CallFunction|ConsumeStamina (Variables|Default|GetSprintCost))))

(event Custom|End%20Damage%20Trace
  ;[0.15 0.15 0.15] Sword Traces
  (if (Utilities|Time|IsValidTimerHandle (stale Custom|Begin%20Damage%20Trace _returnvalue))
    (Utilities|Time|ClearandInvalidateTimerbyHandle (stale Custom|Begin%20Damage%20Trace _returnvalue))))

(event Custom|Begin%20Damage%20Trace
  ;[0.15 0.15 0.15] Sword Traces
  (bind _returnvalue (Utilities|Time|SetTimerbyEvent (delegate Custom|Damage%20Trace) 0.01 true)))

(event Custom|Damage%20Trace
  (bind _playerbp (Variables|Default|GetPlayerBP))
  ;[0.15 0.15 0.15] Sword Traces
  (bind (_outhit _returnvalue) (Collision|SphereTraceForObjects (Transformation|GetWorldLocation (Variables|/Game/Danny/DannyBlueprints/BP_ThirdPersonCharacter.BP_ThirdPersonCharacter_C|GetStart%20Sword%20Trace%20Pos _playerbp)) (Transformation|GetWorldLocation (Variables|/Game/Danny/DannyBlueprints/BP_ThirdPersonCharacter.BP_ThirdPersonCharacter_C|GetEnd%20Sword%20Trace%20Pos _playerbp)) 1e+01 (Utilities|Array|MakeArray "ObjectTypeQuery3") false 0 "ForOneFrame"))
  (if _returnvalue
    (Utilities|FlowControl|DoOnce false :!label _label
      (:Completed
        (Game|Damage|ApplyDamage (.HitActor (Collision|BreakHitResult _outhit)) (Variables|Default|GetSword%20Damage) 0 0)
        (Utilities|FlowControl|Delay 0.3)
        (goto _label Reset)))))

(event Input|EnhancedActionEvents|EnhancedInputActionIA_LockOn
  (params (ActionValue :type Boolean) (ElapsedSeconds :type Float%20%28double-precision%29) (TriggeredSeconds :type Float%20%28double-precision%29) (InputAction :type Input%20Action%20Object%20Reference :default "/Game/Danny/DannyInputActions/IA_LockOn.IA_LockOn"))
  (bind _returnvalue (Game|GetPlayerCameraManager 0))
  (bind _playerbp (Variables|Default|GetPlayerBP))
  (bind _playerbp_2 (Variables|Default|GetPlayerBP))
  (bind _transformcomponent (Variables|/Script/Engine.PlayerCameraManager|GetTransformComponent _returnvalue))
  (bind _charactermovement (Variables|/Script/Engine.Character|GetCharacterMovement _playerbp))
  (bind _charactermovement_2 (Variables|/Script/Engine.Character|GetCharacterMovement _playerbp_2))
  (bind _returnvalue_2 (Transformation|GetWorldLocation _transformcomponent))
  ;[0.15 0.15 0.15] Target Lock
  (:Started
    (Variables|Default|GetTargetLockActor
      (:then
        ;;[0.15 0.15 0.15 0.5] Turn off LockOn if active
        (Variables|Default|SetTargetLockActor 0)
        (Variables|/Script/Engine.CharacterMovementComponent|SetbOrientRotationToMovement _charactermovement true)
        (Variables|/Script/Engine.CharacterMovementComponent|SetbUseControllerDesiredRotation _charactermovement false)
        (Actor|DestroyActor (Variables|Default|GetTargetLockWidget)))
      (:else
        (bind (_outhit _returnvalue_3) (Collision|SphereTraceForObjects "0, 0, 0" (+ (Math|Vector|MakeVector (.x _returnvalue_2) (.y _returnvalue_2) (+ (.z _returnvalue_2) 2e+01)) (* (Math|Vector|GetForwardVector (Transformation|GetWorldRotation _transformcomponent)) 1e+03)) 2.5e+02 (Utilities|Array|MakeArray "ObjectTypeQuery3") false 0 "ForDuration" true "(R=1.000000,G=0.000000,B=0.000000,A=1.000000)" "(R=0.000000,G=1.000000,B=0.000000,A=1.000000)" 2.0))
        (if _returnvalue_3
          (Variables|Default|SetTargetLockActor (.HitActor (Collision|BreakHitResult _outhit)))
          (Variables|/Script/Engine.CharacterMovementComponent|SetbOrientRotationToMovement _charactermovement_2 false)
          (Variables|/Script/Engine.CharacterMovementComponent|SetbUseControllerDesiredRotation _charactermovement_2 true)
          (bind _returnvalue_4 (Game|SpawnActorfromClass "/Game/Danny/DannyBlueprints/BP_TargetLockWidget.BP_TargetLockWidget_C" (Math|Transform|MakeTransform (Math|Vector|MakeVector (.x (.location (Transformation|GetActorTransform (Variables|Default|GetTargetLockActor)))) (.y (.location (Transformation|GetActorTransform (Variables|Default|GetTargetLockActor)))) (+ (.z (.location (Transformation|GetActorTransform (Variables|Default|GetTargetLockActor)))) 2e+01)) (.rotation (Transformation|GetActorTransform (Variables|Default|GetTargetLockActor))) "1.000000,1.000000,1.000000") "AlwaysSpawn" "MultiplyWithRoot" 0 0))
          (bind _output_get (Variables|Default|SetTargetLockWidget _returnvalue_4))
          (Transformation|AttachActorToActor _output_get (Variables|Default|GetTargetLockActor) "None" "SnapToTarget" "SnapToTarget" "SnapToTarget" true))))))

(event Input|EnhancedActionEvents|EnhancedInputActionIA_Attack
  (params (ActionValue :type Boolean) (ElapsedSeconds :type Float%20%28double-precision%29) (TriggeredSeconds :type Float%20%28double-precision%29) (InputAction :type Input%20Action%20Object%20Reference :default "/Game/Danny/DannyInputActions/IA_Attack.IA_Attack"))
  ;[0.15 0.15 0.15] Sword Combo Animation
  (:Started
    (if (not (Variables|Default|GetIsAttacking?))
      (Variables|Default|SetIsAttacking? true)
      (Animation|Montage|PlayMontage (Variables|/Script/Engine.Character|GetMesh (Variables|Default|GetPlayerBP)) "/Game/Placeholder_Assets/Placeholder_Animations/Combat/SwordAttackCombo_Montage.SwordAttackCombo_Montage"
        (:OnCompleted
          (Variables|Default|SetIsAttacking? false :!label _label)
          (Variables|Default|SetCombo? false))
        (:OnInterrupted
          (goto _label))
        (:OnNotifyBegin
          (if (and (Variables|Default|GetIsAttacking?) (Variables|Default|GetCombo?))
            (Variables|Default|SetCombo? false)
            (else
              (Animation|Montage|MontageStop (Components|SkeletalMesh|GetAnimInstance (Variables|/Script/Engine.Character|GetMesh (Variables|Default|GetPlayerBP))) 0.2 "/Game/Placeholder_Assets/Placeholder_Animations/Combat/SwordAttackCombo_Montage.SwordAttackCombo_Montage")))))
      (else
        (Variables|Default|SetCombo? true)))))

(event EventTick
  (params (DeltaSeconds :type Float%20%28single-precision%29))
  (bind _playerbp (Variables|Default|GetPlayerBP))
  (bind _targetlockactor (Variables|Default|GetTargetLockActor))
  (bind _returnvalue (Transformation|GetActorLocation _playerbp))
  (bind _returnvalue_2 (Transformation|GetActorLocation _targetlockactor))
  (bind _returnvalue_3 (Math|Rotator|FindLookatRotation _returnvalue _returnvalue_2))
  ;[0.15 0.15 0.15] Target Lock
  ;;[0.15 0.15 0.15] Target Lock Update
  (Variables|Default|GetTargetLockActor
    (:then
      (Pawn|SetControlRotation (Pawn|GetController (Variables|Default|GetPlayerBP)) (Math|Rotator|MakeRotator (.roll _returnvalue_3) (+ (.pitch _returnvalue_3) -2e+01) (.yaw _returnvalue_3)))
      (bind _asbp_third_person_character (Utilities|Casting|CastToBP_ThirdPersonCharacter (Game|GetPlayerCharacter 0)))
      (if (Variables|/Game/Danny/DannyBlueprints/BP_ThirdPersonCharacter.BP_ThirdPersonCharacter_C|GetIsSprinting _asbp_third_person_character)
        _))
    (:else)))

(event EventBeginPlay
  ;[0.15 0.15 0.15] Set Player Class
  (bind _asbp_third_person_character (Utilities|Casting|CastToBP_ThirdPersonCharacter (Components|GetOwner)))
  (Variables|Default|SetPlayerBP _asbp_third_person_character))

(fn ConsumeStamina
  (params (Amount :type Float%20%28double-precision%29))
  (bind _output_get (Variables|Default|SetCurrentStamina (Math|Float|Clamp(Float) (Utilities|Operators|Subtract (Variables|Default|GetCurrentStamina) Amount) 0.0 (Variables|Default|GetMaxStamina))))
  (if (<= (Variables|Default|GetCurrentStamina) 0.0)
    (Variables|Default|SetIsExhausted true))
  (Development|PrintString (Utilities|String|ToString(Float) _output_get)))