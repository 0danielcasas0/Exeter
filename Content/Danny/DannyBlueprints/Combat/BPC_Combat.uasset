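; Player combat component for BP_ThirdPersonCharacter, handling stamina-gated dodges and sword combo attacks.
; Dodge picks a directional montage from the last direction key when using controller rotation, otherwise forward.
; Attack presses during a swing queue a combo; montage notifies continue it or stop it, spending stamina and pausing regeneration.
; Begin/EndDamageTrace run a looping-timer sphere trace along the blade, applying damage with a short re-hit cooldown.
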(event Custom|End%20Damage%20Trace
  ;[0.15 0.15 0.15] Sword Traces
  (if (Utilities|Time|IsValidTimerHandle (stale Custom|Begin%20Damage%20Trace _returnvalue))
    (Utilities|Time|ClearandInvalidateTimerbyHandle (stale Custom|Begin%20Damage%20Trace _returnvalue))))

(event Custom|Begin%20Damage%20Trace
  ;[0.15 0.15 0.15] Sword Traces
  (bind _returnvalue (Utilities|Time|SetTimerbyEvent (delegate Custom|Damage%20Trace) 0.01 true)))

(event Custom|Damage%20Trace
  (bind _playerbp (Variables|Default|GetPlayerBP))
  ;[0.15 0.15 0.15] Sword Traces
  (bind (_outhit _returnvalue) (Collision|SphereTraceForObjects (Transformation|GetWorldLocation (Variables|/Game/Danny/DannyBlueprints/BP_ThirdPersonCharacter.BP_ThirdPersonCharacter_C|GetStart%20Sword%20Trace%20Pos _playerbp)) (Transformation|GetWorldLocation (Variables|/Game/Danny/DannyBlueprints/BP_ThirdPersonCharacter.BP_ThirdPersonCharacter_C|GetEnd%20Sword%20Trace%20Pos _playerbp)) 1e+01 (Utilities|Array|MakeArray "ObjectTypeQuery3") false 0 "ForOneFrame"))
  (if _returnvalue
    (Utilities|FlowControl|DoOnce false :!label _label
      (:Completed
        (Game|Damage|ApplyDamage (.HitActor (Collision|BreakHitResult _outhit)) (Variables|Default|GetSword%20Damage) 0 0)
        (Utilities|FlowControl|Delay 0.3)
        (goto _label Reset)))))

(event Input|EnhancedActionEvents|EnhancedInputActionIA_Attack
  (params (ActionValue :type Boolean) (ElapsedSeconds :type Float%20%28double-precision%29) (TriggeredSeconds :type Float%20%28double-precision%29) (InputAction :type Input%20Action%20Object%20Reference :default "/Game/Danny/DannyInputActions/IA_Attack.IA_Attack"))
  (bind _playerbp (Variables|Default|GetPlayerBP))
  (bind _bpc_stats (Variables|/Game/Danny/DannyBlueprints/BP_ThirdPersonCharacter.BP_ThirdPersonCharacter_C|GetBPC_Stats _playerbp))
  ;[0.15 0.15 0.15] Sword Combo Animation
  (:Started
    (if (and (not (Variables|Default|GetIsAttacking?)) (>= (Variables|/Game/Danny/DannyBlueprints/BPC_Stats.BPC_Stats_C|GetStamina (Variables|/Game/Danny/DannyBlueprints/BP_ThirdPersonCharacter.BP_ThirdPersonCharacter_C|GetBPC_Stats (Variables|Default|GetPlayerBP))) 1e+01))
      (Variables|Default|SetIsAttacking? true)
      (Animation|Montage|PlayMontage (Variables|/Script/Engine.Character|GetMesh (Variables|Default|GetPlayerBP)) "/Game/Placeholder_Assets/Placeholder_Animations/Combat/SwordAttackCombo_Montage.SwordAttackCombo_Montage"
        (:then
          (Variables|/Game/Danny/DannyBlueprints/BPC_Stats.BPC_Stats_C|SetregainStamina? (Variables|/Game/Danny/DannyBlueprints/BP_ThirdPersonCharacter.BP_ThirdPersonCharacter_C|GetBPC_Stats (Variables|Default|GetPlayerBP)) false))
        (:OnCompleted
          (Variables|Default|SetIsAttacking? false :!label _label)
          (Variables|Default|SetCombo? false)
          (Variables|/Game/Danny/DannyBlueprints/BPC_Stats.BPC_Stats_C|SetregainStamina? _bpc_stats true)
          (Default|IncreaseValue _bpc_stats "NewEnumerator1" -1e+01 :!label _label_2))
        (:OnInterrupted
          (goto _label))
        (:OnNotifyBegin
          (if (Math|Boolean|ANDBoolean (Variables|Default|GetIsAttacking?) (Variables|Default|GetCombo?) (>= (Variables|/Game/Danny/DannyBlueprints/BPC_Stats.BPC_Stats_C|GetStamina (Variables|/Game/Danny/DannyBlueprints/BP_ThirdPersonCharacter.BP_ThirdPersonCharacter_C|GetBPC_Stats (Variables|Default|GetPlayerBP))) 1e+01))
            (Variables|Default|SetCombo? false)
            (goto _label_2)
            (else
              (Animation|Montage|MontageStop (Components|SkeletalMesh|GetAnimInstance (Variables|/Script/Engine.Character|GetMesh (Variables|Default|GetPlayerBP))) 0.2 "/Game/Placeholder_Assets/Placeholder_Animations/Combat/SwordAttackCombo_Montage.SwordAttackCombo_Montage")))))
      (else
        (Variables|Default|SetCombo? true)))))

(event Input|EnhancedActionEvents|EnhancedInputActionIA_Dodge
  (params (ActionValue :type Boolean) (ElapsedSeconds :type Float%20%28double-precision%29) (TriggeredSeconds :type Float%20%28double-precision%29) (InputAction :type Input%20Action%20Object%20Reference :default "/Game/Danny/DannyInputActions/IA_Dodge.IA_Dodge"))
  (bind _playerbp (Variables|Default|GetPlayerBP))
  (bind _bpc_stats (Variables|/Game/Danny/DannyBlueprints/BP_ThirdPersonCharacter.BP_ThirdPersonCharacter_C|GetBPC_Stats _playerbp))
  ;[0.15 0.15 0.15] Dodging
  (:Started
    (if (and (not (Variables|Default|GetIsDodging?)) (>= (Variables|/Game/Danny/DannyBlueprints/BPC_Stats.BPC_Stats_C|GetStamina (Variables|/Game/Danny/DannyBlueprints/BP_ThirdPersonCharacter.BP_ThirdPersonCharacter_C|GetBPC_Stats (Variables|Default|GetPlayerBP))) 25.0))
      (Variables|Default|SetIsDodging? true)
      (Utilities|FlowControl|Sequence
        (:then_0
          (if (Variables|/Script/Engine.CharacterMovementComponent|GetbUseControllerDesiredRotation (Variables|/Script/Engine.Character|GetCharacterMovement (Variables|Default|GetPlayerBP)))
            (switch string (Utilities|String|ToString(Text) (Class|KismetInputLibrary|KeyGetDisplayName (Variables|/Game/Danny/DannyBlueprints/BP_ThirdPersonCharacter.BP_ThirdPersonCharacter_C|GetDirection%20Key (Variables|Default|GetPlayerBP)) true))
              (:W
                (Variables|Default|SetmovementDIrection "NewEnumerator0"))
              (:A
                (Variables|Default|SetmovementDIrection "NewEnumerator1"))
              (:S
                (Variables|Default|SetmovementDIrection "NewEnumerator2"))
              (:D
                (Variables|Default|SetmovementDIrection "NewEnumerator3")))
            (else
              (Variables|Default|SetmovementDIrection "NewEnumerator0"))))
        (:then_1
          (Animation|Montage|PlayMontage (Variables|/Script/Engine.Character|GetMesh (Variables|Default|GetPlayerBP)) (Utilities|Select :Index (Variables|Default|GetmovementDIrection) :NewEnumerator0 "/Game/Placeholder_Assets/Placeholder_Animations/Dodge/Dodge_F_Montage.Dodge_F_Montage" :NewEnumerator1 "/Game/Placeholder_Assets/Placeholder_Animations/Dodge/Dodge_L_Montage.Dodge_L_Montage" :NewEnumerator2 "/Game/Placeholder_Assets/Placeholder_Animations/Dodge/Dodge_B_Montage.Dodge_B_Montage" :NewEnumerator3 "/Game/Placeholder_Assets/Placeholder_Animations/Dodge/Dodge_R_Montage.Dodge_R_Montage") 1.2 0.0 "None" false
            (:then
              (Variables|/Game/Danny/DannyBlueprints/BPC_Stats.BPC_Stats_C|SetregainStamina? _bpc_stats false)
              (Default|IncreaseValue _bpc_stats "NewEnumerator1" -25.0))
            (:OnCompleted
              (Variables|Default|SetIsDodging? false :!label _label)
              (Variables|/Game/Danny/DannyBlueprints/BPC_Stats.BPC_Stats_C|SetregainStamina? (Variables|/Game/Danny/DannyBlueprints/BP_ThirdPersonCharacter.BP_ThirdPersonCharacter_C|GetBPC_Stats (Variables|Default|GetPlayerBP)) true))
            (:OnInterrupted
              (goto _label))))))))

(event EventBeginPlay
  ;[0.15 0.15 0.15] Set Player Class
  (bind _asbp_third_person_character (Utilities|Casting|CastToBP_ThirdPersonCharacter (Components|GetOwner)))
  (Variables|Default|SetPlayerBP _asbp_third_person_character))