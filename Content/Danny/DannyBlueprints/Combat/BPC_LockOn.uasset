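; Player lock-on component for BP_ThirdPersonCharacter that toggles targeting of enemies with IA_LockOn.
; A sphere trace from player toward camera aim locks the first "Enemy"-tagged pawn, attaches a BP_TargetLockWidget and switches movement to controller-facing rotation.
; Tick steers control rotation at the target with a downward pitch offset.
; Target death releases the lock like toggling off, but leaves the temporary LockedOn flag set.
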(event Input|EnhancedActionEvents|EnhancedInputActionIA_LockOn
  (params (ActionValue :type Boolean) (ElapsedSeconds :type Float%20%28double-precision%29) (TriggeredSeconds :type Float%20%28double-precision%29) (InputAction :type Input%20Action%20Object%20Reference :default "/Game/Danny/DannyInputActions/IA_LockOn.IA_LockOn"))
  (bind _returnvalue (Game|GetPlayerCameraManager 0))
  (bind _playerbp (Variables|Default|GetPlayerBP))
  (bind _playerbp_2 (Variables|Default|GetPlayerBP))
  (bind _transformcomponent (Variables|/Script/Engine.PlayerCameraManager|GetTransformComponent _returnvalue))
  (bind _charactermovement (Variables|/Script/Engine.Character|GetCharacterMovement _playerbp))
  (bind _charactermovement_2 (Variables|/Script/Engine.Character|GetCharacterMovement _playerbp_2))
  (bind _returnvalue_2 (Transformation|GetWorldLocation _transformcomponent))
  ;[0.15 0.15 0.15] Target Lock
  (:Started
    (Variables|Default|GetTargetLockActor
      (:then
        ;;[0.15 0.15 0.15 0.5] Turn off LockOn if active
        (Variables|Default|SetTargetLockActor 0)
        (Variables|Default|SetLockedOn? false) ; TEMPORARY
        (Variables|/Script/Engine.CharacterMovementComponent|SetbOrientRotationToMovement _charactermovement true)
        (Variables|/Script/Engine.CharacterMovementComponent|SetbUseControllerDesiredRotation _charactermovement false)
        (Actor|DestroyActor (Variables|Default|GetTargetLockWidget)))
      (:else
        (bind _outhits (Collision|MultiSphereTraceForObjects (Transformation|GetActorLocation (Variables|Default|GetPlayerBP)) (+ (Math|Vector|MakeVector (.x _returnvalue_2) (.y _returnvalue_2) (.z _returnvalue_2)) (* (Math|Vector|GetForwardVector (Transformation|GetWorldRotation _transformcomponent)) 1.5e+03)) 3e+02 (Utilities|Array|MakeArray "ObjectTypeQuery3") false 0 "ForOneFrame"))
        (bind _array_element (Utilities|Array|ForEachLoopwithBreak _outhits :!label _label)
          (:LoopBody
            (if (Actor|ActorHasTag (.HitActor (Collision|BreakHitResult _array_element)) "Enemy")
              (Variables|Default|SetTargetLockActor (.HitActor (Collision|BreakHitResult _array_element)))
              (Variables|/Script/Engine.CharacterMovementComponent|SetbOrientRotationToMovement _charactermovement_2 false)
              (Variables|/Script/Engine.CharacterMovementComponent|SetbUseControllerDesiredRotation _charactermovement_2 true)
              (Variables|Default|SetLockedOn? true :!pinned true) ; TEMPORARY
              (bind _returnvalue_3 (Game|SpawnActorfromClass "/Game/Danny/DannyBlueprints/Combat/BP_TargetLockWidget.BP_TargetLockWidget_C" (Math|Transform|MakeTransform (Math|Vector|MakeVector (.x (.location (Transformation|GetActorTransform (Variables|Default|GetTargetLockActor)))) (.y (.location (Transformation|GetActorTransform (Variables|Default|GetTargetLockActor)))) (+ (.z (.location (Transformation|GetActorTransform (Variables|Default|GetTargetLockActor)))) 2e+01)) (.rotation (Transformation|GetActorTransform (Variables|Default|GetTargetLockActor))) "1.000000,1.000000,1.000000") "AlwaysSpawn" "MultiplyWithRoot" 0 0))
              (bind _output_get (Variables|Default|SetTargetLockWidget _returnvalue_3))
              (Transformation|AttachActorToActor _output_get (Variables|Default|GetTargetLockActor) "None" "SnapToTarget" "SnapToTarget" "SnapToTarget" true)
              (goto _label Break))))))))

(event EventTick
  (params (DeltaSeconds :type Float%20%28single-precision%29))
  (bind _playerbp (Variables|Default|GetPlayerBP))
  (bind _charactermovement (Variables|/Script/Engine.Character|GetCharacterMovement _playerbp))
  ;[0.15 0.15 0.15] LookAtTarget
  (bind _targetlockactor (Variables|Default|GetTargetLockActor)
    (:then
      (Pawn|SetControlRotation (Pawn|GetController (Variables|Default|GetPlayerBP)) (Math|Rotator|MakeRotator (.roll (Math|Rotator|FindLookatRotation (Transformation|GetActorLocation (Variables|Default|GetPlayerBP)) (Transformation|GetActorLocation _targetlockactor))) (+ (.pitch (Math|Rotator|FindLookatRotation (Transformation|GetActorLocation (Variables|Default|GetPlayerBP)) (Transformation|GetActorLocation _targetlockactor))) -25.0) (.yaw (Math|Rotator|FindLookatRotation (Transformation|GetActorLocation (Variables|Default|GetPlayerBP)) (Transformation|GetActorLocation _targetlockactor)))))
      (bind _asbp_enemy_character (Utilities|Casting|CastToBP_EnemyCharacter _targetlockactor))
      (if (Variables|/Game/Danny/DannyAI/BP_EnemyCharacter.BP_EnemyCharacter_C|GetisDead? _asbp_enemy_character)
        (Variables|Default|SetTargetLockActor 0)
        (Variables|/Script/Engine.CharacterMovementComponent|SetbOrientRotationToMovement _charactermovement true)
        (Variables|/Script/Engine.CharacterMovementComponent|SetbUseControllerDesiredRotation _charactermovement false)
        (Actor|DestroyActor (Variables|Default|GetTargetLockWidget))))
    (:else)))

(event EventBeginPlay
  (bind _asbp_third_person_character (Utilities|Casting|CastToBP_ThirdPersonCharacter (Components|GetOwner)))
  (Variables|Default|SetPlayerBP _asbp_third_person_character))