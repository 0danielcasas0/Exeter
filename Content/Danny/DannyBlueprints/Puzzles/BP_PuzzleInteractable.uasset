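; Interactable actor that opens a grid puzzle widget when the player interacts with it.
; Interact disables further interaction, adds the widget to the viewport and switches to UI-only input with the mouse cursor shown.
; It calls OnPuzzleCompleteMessage on PuzzleManager as soon as the widget opens, not on solve.
; The widget's OnClosed binding only re-enables interaction, and focus events just print debug strings.
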(event Custom|PuzzleClosed
  ;[0.15 0.15 0.15] turns on the ui popup for the interactable on close
  (Variables|Default|SetCanInteract? true))

(event EventInteract
  (params (Interactor :type Actor%20Object%20Reference))
  (bind _returnvalue (Game|GetPlayerController 0))
  (Variables|Default|SetCanInteract? false)
  (Utilities|IsValid "/Game/Danny/DannyUI/PuzzleUI/WBP_GridPuzzle.WBP_GridPuzzle"
    (:Is%20Valid
      (bind _returnvalue_2 (UserInterface|CreateWidget "/Game/Danny/DannyUI/PuzzleUI/WBP_GridPuzzle.WBP_GridPuzzle_C" _returnvalue))
      ;[0.15 0.15 0.15] turns on the ui popup for the interactable on close
      (EventDispatchers|BindEventtoOnClosed _returnvalue_2 (delegate Custom|PuzzleClosed))
      (UserInterface|Viewport|AddtoViewport _returnvalue_2 0)
      (Input|SetInputModeUIOnly _returnvalue _returnvalue_2 "DoNotLock" false)
      (Variables|/Script/Engine.PlayerController|SetbShowMouseCursor _returnvalue true)
      (Class|BPIPuzzle|OnPuzzleComplete(Message) (Variables|Default|GetPuzzleManager)))))

(event EventOnBeginFocus
  (params (Interactor :type Actor%20Object%20Reference))
  (Development|PrintString "Focused"))

(event EventOnEndFocus
  (params (Interactor :type Actor%20Object%20Reference))
  (Development|PrintString "Unfocused"))

(fn ConstructionScript)

(fn CanInteract
  (params (Interactor :type Actor%20Object%20Reference))
  (if (Variables|Default|GetCanInteract?)
    (return true)))

(fn GetInteractionText
  ;[0.15 0.15 0.15] Changes text on interactable hover
  (return "Interact"))