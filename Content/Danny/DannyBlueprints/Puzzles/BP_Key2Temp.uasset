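; BP_Key2Temp is an interactable key pickup that grants its key type to whoever picks it up.
; The construction script passes the key mesh, key map and key type to SetKey to configure the key.
; On interact, it sends the key type through BPI_PlayerKeys and destroys itself, only if the interactor implements that interface.
; It is always interactable with "Pick Up" text, and interact and focus events print debug strings.
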(event EventInteract
  (params (Interactor :type Actor%20Object%20Reference))
  (Development|PrintString "Hello")
  (bind _output_get (Variables|Default|SetOtherActor Interactor))
  (if (Utilities|DoesObjectImplementInterface _output_get "/Game/Danny/DannyBlueprints/BPI_PlayerKeys.BPI_PlayerKeys_C")
    (Class|BPIPlayerKeys|AddKey(Message) (Variables|Default|GetOtherActor) (Variables|Setup|GetKeyType))
    (Actor|DestroyActor)))

(event EventOnBeginFocus
  (params (Interactor :type Actor%20Object%20Reference))
  (Development|PrintString "Focused"))

(event EventOnEndFocus
  (params (Interactor :type Actor%20Object%20Reference))
  (Development|PrintString "Unfocused"))

(fn ConstructionScript
  (CallFunction|SetKey (Utilities|Array|MakeArray (Variables|Default|GetKeyMesh)) (Variables|Default|GetKeyMap) (Variables|Setup|GetKeyType)))

(fn CanInteract
  (params (Interactor :type Actor%20Object%20Reference))
  (return true))

(fn GetInteractionText
  (return "Pick Up"))