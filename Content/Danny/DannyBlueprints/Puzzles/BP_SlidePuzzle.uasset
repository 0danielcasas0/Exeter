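; Interactable sliding-puzzle actor that builds a square tile board at BeginPlay from one texture.
; SpawnPuzzle adds a box component per grid cell and a mesh tile in all but the last, leaving the gap.
; Each tile gets a dynamic material with a UV offset showing its slice of the image.
; Interacting once blends the camera to the puzzle, disables movement and switches to UI-only mouse input; tile sliding is not implemented here.
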(event EventBeginPlay
  (CallFunction|SpawnPuzzle))

(event EventOnBeginFocus
  (params (Interactor :type Actor%20Object%20Reference))
  (Development|PrintString "Puzzle Focused"))

(event EventInteract
  (params (Interactor :type Actor%20Object%20Reference))
  (bind _returnvalue (Game|GetPlayerController 0))
  (if (Variables|Default|GetCanInteract?)
    (Game|Player|SetViewTargetwithBlend _returnvalue self 1.5 "VTBlend_EaseInOut" 2.0 false)
    (Variables|Default|SetCanInteract? false)
    (Pawn|Components|CharacterMovement|DisableMovement (Variables|/Script/Engine.Character|GetCharacterMovement (Game|GetPlayerCharacter 0)))
    (Input|SetInputModeUIOnly _returnvalue 0 "DoNotLock" false)
    (Variables|/Script/Engine.PlayerController|SetbShowMouseCursor _returnvalue true)))

(fn ConstructionScript)

(fn SpawnPuzzle
  (bind _gridsize (Variables|Default|GetGridSize))
  (bind _mesh_size (Variables|Default|GetMesh%20Size))
  (bind _gridsize_2 (Variables|Default|GetGridSize))
  (bind _mesh_size_2 (Variables|Default|GetMesh%20Size))
  (bind _mesh_size_3 (Variables|Default|GetMesh%20Size))
  (bind _gridsize_3 (Variables|Default|GetGridSize))
  (bind _returnvalue (Math|Conversions|ToFloat(Integer) _gridsize_2))
  (bind _returnvalue_2 (- _gridsize 1))
  (bind _returnvalue_3 (/ _mesh_size_3 4.0))
  (bind _returnvalue_4 (- _gridsize_3 1))
  (bind _returnvalue_5 (/ 3.0 _returnvalue))
  (for _index (range 0 _returnvalue_2)
    (Variables|Default|SetY%20Index _index)
    (for _index_2 (range 0 _returnvalue_2)
      (Variables|Default|SetX%20Index _index_2)
      (bind _returnvalue_6 (AddComponent|AddBoxComponent false (Math|Transform|MakeTransform (Math|Vector|MakeVector (* (Variables|Default|GetX%20Index) _mesh_size) (* (Variables|Default|GetY%20Index) _mesh_size) 0.0) "0, 0, 0" "1.000000,1.000000,1.000000")))
      (Components|Box|SetBoxExtent _returnvalue_6 (Math|Vector|MakeVector _returnvalue_3 _returnvalue_3 _returnvalue_3) true)
      (Utilities|Array|Add (Variables|Default|GetSpacesList) _returnvalue_6)
      (if (not (and (== (Variables|Default|GetX%20Index) _returnvalue_4) (== _returnvalue_4 (Variables|Default|GetY%20Index))))
        (bind _returnvalue_7 (AddComponent|AddStaticMeshComponent false (Math|Transform|MakeTransform (Math|Vector|MakeVector (* (Variables|Default|GetX%20Index) _mesh_size_2) (* (Variables|Default|GetY%20Index) _mesh_size_2) 0.0) "0, 0, 0" "0.950000,0.950000,0.950000")))
        (Utilities|Array|Add (Variables|Default|GetMeshesList) _returnvalue_7)
        (bind _returnvalue_8 (Rendering|Material|CreateDynamicMaterialInstance _returnvalue_7 0 "/Game/Danny/DannyBlueprints/Puzzles/M_PuzzleMaterial.M_PuzzleMaterial" "None" :!class /Script/Engine.PrimitiveComponent))
        (Rendering|Material|SetTextureParameterValue _returnvalue_8 "PuzzleTexture" (Variables|Default|GetTexture))
        (Rendering|Material|SetVectorParameterValueonMaterials _returnvalue_7 "TextureOffset2D" (Math|Vector|MakeVector (* (Variables|Default|GetX%20Index) _returnvalue_5) (* (Variables|Default|GetY%20Index) _returnvalue_5) _returnvalue_5))))))

(fn CanInteract
  (params (Interactor :type Actor%20Object%20Reference))
  (return true))

(fn GetInteractionText
  (return "Interact"))