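; BP_NPC is an interactable, ghost-like NPC that bobs in the air and offers a "Speak" prompt to start dialogue.
; Starting dialogue teleports the player to PlayerMark facing the NPC, blends the view to the NPC, swaps player input for cursor UI and shows WBP_DIalogue; EndDialogue restores control.
; A timeline drives the float, while Tick eases mesh yaw toward a player within DetectionRadius, otherwise back to its original rotation.
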(event Custom|StartDialogue
  (params (PlayerChar :type Actor%20Object%20Reference))
  (bind _returnvalue (Game|GetPlayerController 0))
  (bind _playermark (Variables|Default|GetPlayerMark))
  (bind _returnvalue_2 (Transformation|GetWorldLocation _playermark))
  ;[0.15 0.15 0.15] Dialogue
  (Transformation|SetActorLocationAndRotation PlayerChar _returnvalue_2 (Math|Rotator|FindLookatRotation _returnvalue_2 (Transformation|GetActorLocation)) false true)
  (Game|Player|SetViewTargetwithBlend _returnvalue self 0.0 "VTBlend_Linear" 0.0 false)
  (Input|DisableInput PlayerChar _returnvalue)
  (Variables|/Script/Engine.PlayerController|SetbShowMouseCursor _returnvalue true)
  (Input|SetInputModeGameandUI _returnvalue 0 "DoNotLock" true false)
  (bind _returnvalue_3 (UserInterface|CreateWidget "/Game/Danny/DannyUI/DialogueUI/WBP_DIalogue.WBP_DIalogue_C" 0 self))
  (bind _output_get (Variables|Default|SetDialogueWidget _returnvalue_3))
  (UserInterface|Viewport|AddtoViewport _output_get 0))

(event Custom|EndDialogue
  (params (PlayerChar :type Actor%20Object%20Reference))
  (bind _returnvalue (Game|GetPlayerController 0))
  ;[0.15 0.15 0.15] Dialogue
  (Widget|RemovefromParent (Variables|Default|GetDialogueWidget))
  (Game|Player|SetViewTargetwithBlend _returnvalue (Game|GetPlayerCharacter 0) 0.0 "VTBlend_Linear" 0.0 false)
  (Input|EnableInput PlayerChar _returnvalue)
  (Variables|/Script/Engine.PlayerController|SetbShowMouseCursor _returnvalue false)
  (Input|SetInputModeGameOnly _returnvalue false))

(event EventBeginPlay
  (Variables|Default|SetOriginalRotation (Transformation|GetWorldRotation (Variables|Character|GetMesh)))
  ;[0.15 0.15 0.15] Ghost Float
  (Variables|Default|SetBaseLocation (Transformation|GetRelativeTransform (Variables|Character|GetMesh)))
  (bind _bobalpha (Timeline|GhostFloatTimeline PlayFromStart)
    (:Update
      (Transformation|SetRelativeLocation (Variables|Character|GetMesh) (Math|Vector|MakeVector (.x (.Location (Math|Transform|BreakTransform (Variables|Default|GetBaseLocation)))) (.y (.Location (Math|Transform|BreakTransform (Variables|Default|GetBaseLocation)))) (+ (.z (.Location (Math|Transform|BreakTransform (Variables|Default|GetBaseLocation)))) (* _bobalpha (Variables|Default|GetFloatHeight)))) false false))))

(event EventTick
  (params (DeltaSeconds :type Float%20%28single-precision%29))
  (bind _returnvalue (Game|GetPlayerCharacter 0))
  (bind _mesh (Variables|Character|GetMesh))
  (bind _mesh_2 (Variables|Character|GetMesh))
  (if (< (Transformation|GetDistanceTo _returnvalue) (Variables|Default|GetDetectionRadius))
    (Transformation|SetWorldRotation _mesh (Math|Interpolation|RInterpTo (Transformation|GetWorldRotation _mesh_2) (Math|Rotator|MakeRotator 0.0 0.0 (+ (.Yaw (Math|Rotator|BreakRotator (Math|Rotator|FindLookatRotation (Transformation|GetWorldLocation _mesh_2) (Transformation|GetActorLocation _returnvalue)))) -9e+01)) DeltaSeconds 2.0) false false)
    (else
      (Transformation|SetWorldRotation _mesh (Math|Interpolation|RInterpTo (Transformation|GetWorldRotation _mesh) (Variables|Default|GetOriginalRotation) DeltaSeconds 2.0) false false))))

(event EventInteract
  (params (Interactor :type Actor%20Object%20Reference))
  (CallFunction|StartDialogue Interactor))

(fn ConstructionScript)

(fn CanInteract
  (params (Interactor :type Actor%20Object%20Reference))
  (return true))

(fn GetInteractionText
  (return "Speak"))